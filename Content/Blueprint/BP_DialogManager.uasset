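; BP_DialogManager is an Actor Blueprint that steps through an array of dialog lines.
; Its DisplayNextLine event shows the current line with Print Text, then advances the index, wrapping to the first line once the end is reached.
; The file contains no trigger for that event, as BeginPlay, overlap and Tick are unused.
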(event Custom|DisplayNextLine
  (if (>= (Variables|Default|GetIndex) (Utilities|Array|Length (Variables|Default|GetDialog)))
    (Variables|Default|SetIndex 0))
  (Development|PrintText (Utilities|Array|Get(acopy) (Variables|Default|GetDialog) (Variables|Default|GetIndex)))
  (Math|Integer|IncrementInt (Variables|Default|GetIndex)))

(event EventBeginPlay)

(event Collision|EventActorBeginOverlap
  (params (OtherActor :type Actor%20Object%20Reference)))

(event EventTick
  (params (DeltaSeconds :type Float%20%28single-precision%29)))

(fn ConstructionScript)